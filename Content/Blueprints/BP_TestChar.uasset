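; BP_TestChar is a test character with a first-person style camera, look and movement.
; The construction script creates the camera on the mesh's Head socket, with pawn control rotation disabled.
; Each tick, axis key input sets actor yaw and accumulates a clamped pitch value, which is never applied to the camera.
; MoveX and MoveY axes form a normalized direction from actor forward and right vectors to drive movement.
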(event EventBeginPlay
  (Variables|Default|SetLookX (.yaw (Transformation|GetActorRotation)))
  (Variables|Default|SetLookY (.pitch (Transformation|GetWorldRotation (Variables|Default|GetCamera)))))

(event EventTick
  (params (DeltaSeconds :type Float%20%28single-precision%29))
  (bind _looklimit (Variables|Default|GetLookLimit))
  (bind _output_get (Variables|Default|SetLookX (+ (* DeltaSeconds (* (Class|Actor|GetInputAxisKeyValue) (Variables|Default|GetLookSpeed))) (Variables|Default|GetLookX))))
  (Transformation|SetActorRotation (Math|Rotator|MakeRotator 0.0 0.0 _output_get))
  (Variables|Default|SetLookY (Math|Float|Clamp(Float) (+ (Variables|Default|GetLookY) (* DeltaSeconds (* (Class|Actor|GetInputAxisKeyValue) (Variables|Default|GetLookSpeed)))) (* _looklimit -1.0) _looklimit))
  (Pawn|Input|AddMovementInput (Class|KismetMathLibrary|VectorNormal2D (+ (* (Transformation|GetActorForwardVector) (Variables|Default|GetMoveY)) (* (Transformation|GetActorRightVector) (Variables|Default|GetMoveX))) 0.0001) 1.0 false))

(event Input|AxisEvents|InputAxisMoveX
  (params (AxisValue :type Float%20%28single-precision%29))
  (Variables|Default|SetMoveX AxisValue))

(event Input|AxisEvents|InputAxisMoveY
  (params (AxisValue :type Float%20%28single-precision%29))
  (Variables|Default|SetMoveY AxisValue))

(fn ConstructionScript
  (bind _returnvalue (AddComponent|AddCameraComponent true))
  (Transformation|AttachComponentToComponent _returnvalue (Variables|Character|GetMesh) "Head" "KeepRelative" "KeepRelative" "KeepRelative" true)
  (Transformation|SetRelativeLocation _returnvalue "0.000000,-22.000000,8.000000" false false)
  (Transformation|SetRelativeRotation _returnvalue "90.000000,0.000000,-90.000000" false false)
  (bind _output_get (Variables|Default|SetCamera _returnvalue))
  (Variables|/Script/Engine.CameraComponent|SetbUsePawnControlRotation _output_get false))