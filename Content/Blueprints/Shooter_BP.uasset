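; Shooter character Blueprint that adds 2D sound feedback for the player's combat events.
; Melee first hits play a flesh or metal impact depending on whether the struck class derives from AIBase, using a concurrency setting.
; Health damage and death share one hurt sound.
; Combat reload and swap events play sounds taken from the held weapon, with only reload checking that its sound is valid.
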(event OnFirstHit(Melee)
  (params (StruckActor :type Actor%20Object%20Reference) (StruckActorClass :type Object%20Class%20Reference))
  (Audio|PlaySound2D (select (Utilities|ClassIsChildOf StruckActorClass "/Script/UnrealPlayground.AIBase") "/Game/Audio/SFX/Weapon/Wrench/SFX_WPN_WN_Impact_Flesh_.SFX_WPN_WN_Impact_Flesh_" "/Game/Audio/SFX/Weapon/Wrench/SFX_WPN_WN_Impact_Metal_.SFX_WPN_WN_Impact_Metal_") 1.0 1.0 0.0 "/Game/Audio/SFX/PlayOldest.PlayOldest" 0))

(event OnDamaged(Health)
  ;[1 1 1] Take Damage SFX
  (Audio|PlaySound2D "/Game/Audio/SFX/Player/SFX_PL_DamageTaken.SFX_PL_DamageTaken" 7.0 1.0 0.0 0 0))

(event OnDeath(Health)
  ;[1 1 1] Take Damage SFX
  (Audio|PlaySound2D "/Game/Audio/SFX/Player/SFX_PL_DamageTaken.SFX_PL_DamageTaken" 7.0 1.0 0.0 0 0))

(event OnReload(Combat)
  (bind _combat (Variables|Default|GetCombat))
  (bind _returnvalue (Class|CombatComponent|GetHeldWeapon _combat))
  (bind _sfxreload (Variables|/Script/UnrealPlayground.Weapon|GetSFXReload _returnvalue))
  ;[1 1 1] Reload SFX
  (Utilities|IsValid _sfxreload
    (:Is%20Valid
      (Audio|PlaySound2D _sfxreload 0.6 1.0 0.0 0 self))))

(event OnSwap(Combat)
  ;[1 1 1] Swap SFX
  (Audio|PlaySound2D (Variables|/Script/UnrealPlayground.Weapon|GetSFXSwap (Class|CombatComponent|GetHeldWeapon (Variables|Default|GetCombat))) 0.6 1.0 0.0 0 0))

(fn ConstructionScript)