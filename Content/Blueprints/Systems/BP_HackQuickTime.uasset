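; BP_HackQuickTime displays on-screen key prompts for what its name indicates is a hacking quick-time event.
; Its First, Second and Third events each create a WBP_QuickTime widget owned by the Player's ShooterController, add it to the viewport and set its key image to R, C or E respectively.
; Each event caches its widget, and Destroy removes only the most recently cached one; input handling and sequencing are absent here.
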(event Custom|Third
  (bind _returnvalue (UserInterface|CreateWidget "/Game/Blueprints/UI/Widgets/WBP_QuickTime.WBP_QuickTime_C" (.AsShooter%20Controller (Utilities|Casting|CastToShooterController (Pawn|GetController (Variables|Default|GetPlayer))))))
  (UserInterface|Viewport|AddtoViewport _returnvalue 0)
  (Appearance|SetBrushfromTexture (Variables|/Script/ProjectNova.QuickTimeWidget|GetKeyImage _returnvalue) "/Game/Art/Textures/KeyboardKeys/T_Key_E.T_Key_E" false)
  (Variables|Default|SetCache%20Widget _returnvalue))

(event Custom|First
  (bind _returnvalue (UserInterface|CreateWidget "/Game/Blueprints/UI/Widgets/WBP_QuickTime.WBP_QuickTime_C" (.AsShooter%20Controller (Utilities|Casting|CastToShooterController (Pawn|GetController (Variables|Default|GetPlayer))))))
  (UserInterface|Viewport|AddtoViewport _returnvalue 0)
  (Appearance|SetBrushfromTexture (Variables|/Script/ProjectNova.QuickTimeWidget|GetKeyImage _returnvalue) "/Game/Art/Textures/KeyboardKeys/T_Key_R.T_Key_R" false)
  (Variables|Default|SetCache%20Widget _returnvalue))

(event Custom|Second
  (bind _returnvalue (UserInterface|CreateWidget "/Game/Blueprints/UI/Widgets/WBP_QuickTime.WBP_QuickTime_C" (.AsShooter%20Controller (Utilities|Casting|CastToShooterController (Pawn|GetController (Variables|Default|GetPlayer))))))
  (UserInterface|Viewport|AddtoViewport _returnvalue 0)
  (Appearance|SetBrushfromTexture (Variables|/Script/ProjectNova.QuickTimeWidget|GetKeyImage _returnvalue) "/Game/Art/Textures/KeyboardKeys/T_Key_C.T_Key_C" false)
  (Variables|Default|SetCache%20Widget _returnvalue))

(event Custom|Destroy
  (Widget|RemovefromParent (Variables|Default|GetCache%20Widget)))

(event EventBeginPlay)

(fn ConstructionScript)