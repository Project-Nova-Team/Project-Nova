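; BP_EngineerHUD is the HUD Blueprint that creates and routes updates to the player's on-screen widgets.
; BuildBlueprintWidgets creates the interaction prompt, weapon display, pause menu and exit confirmation widgets, stores them and adds all four to the viewport.
; WeaponUpdate passes weapon info to the weapon display.
; InteractionPromptProvided only prints a debug string, as the logic to show, set or hide the prompt is disconnected.
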(event EventBuildBlueprintWidgets
  (bind _playerowner (Variables|Default|GetPlayerOwner))
  ;[1 1 1] Create widgets
  (bind _returnvalue (UserInterface|CreateWidget "/Game/Blueprints/UI/InteractionPrompt.InteractionPrompt_C" _playerowner))
  (bind _output_get (Variables|Default|SetInteractionPromptWidget _returnvalue))
  (UserInterface|Viewport|AddtoViewport _output_get 0)
  (bind _returnvalue_2 (UserInterface|CreateWidget "/Game/Blueprints/UI/WeaponDisplay.WeaponDisplay_C" _playerowner))
  (bind _output_get_2 (Variables|Default|SetWeaponDisplayWidget _returnvalue_2))
  (UserInterface|Viewport|AddtoViewport _output_get_2 0)
  (bind _returnvalue_3 (UserInterface|CreateWidget "/Game/Blueprints/UI/PauseMenu.PauseMenu_C" _playerowner))
  (bind _output_get_3 (Variables|Default|SetPauseMenuWidget _returnvalue_3))
  (UserInterface|Viewport|AddtoViewport _output_get_3 0)
  (bind _returnvalue_4 (UserInterface|CreateWidget "/Game/Blueprints/UI/ExitConfirmation.ExitConfirmation_C" _playerowner))
  (bind _output_get_4 (Variables|Default|SetExitConfirmationWidget _returnvalue_4))
  (UserInterface|Viewport|AddtoViewport _output_get_4 0))

(event EventWeaponUpdate
  (params (Info :type Weapon%20HUD%20Structure%20%28by%20ref%29))
  ;[1 1 1] Weapon HUD
  (bind _asweapon_display (Utilities|Casting|CastToWeaponDisplay (Variables|Default|GetWeaponDisplayWidget)))
  (Default|Update _asweapon_display Info))

(event EventInteractionPromptProvided
  (params (Prompt :type Interaction%20Prompt%20Structure%20%28by%20ref%29))
  (Development|PrintString "Hello"))

(fn ConstructionScript)