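; HallwayGorm is an AI-controlled character that plays a scripted walk down a hallway.
; It caches its AI controller when possessed.
; The WalkDownHall event calls Enable, which makes the mesh visible and orders the controller to move to the location of the TargetPos component.
; A separate FinishWalkDownHall event destroys the actor, and nothing in this graph calls either event.
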(event Custom|WalkDownHall
  (CallFunction|Enable))

(event Custom|FinishWalkDownHall
  (Actor|DestroyActor))

(event EventPossessed
  (params (NewController :type Controller%20Object%20Reference))
  (bind _asaicontroller (Utilities|Casting|CastToAIController NewController))
  (Variables|Default|SetAICont _asaicontroller))

(fn ConstructionScript)

(fn Enable
  (Rendering|SetVisibility (Variables|Character|GetMesh) true false)
  (AI|Navigation|MovetoLocation (Variables|Default|GetAICont) (Transformation|GetWorldLocation (Variables|Default|GetTargetPos)) 2e+01 true true false true 0))