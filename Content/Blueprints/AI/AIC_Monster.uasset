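; AI controller for a monster that sets and clears its Blackboard Target as an enemy is sensed or lost.
; SpotEnemy takes a stimulus, and on successful sensing it cancels the lost-sight timer and stores the enemy as Target.
; A failed stimulus starts a one-shot LoseSightDuration timer whose LostSight event clears Target, giving a grace period before the monster forgets its target.
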(event Custom|Lost%20Sight
  (AI|Components|Blackboard|SetValueasObject (Variables|Default|GetBlackboard) (Variables|Default|GetTarget) 0))

(event EventSpotEnemy
  (params (Enemy :type Actor%20Object%20Reference) (Stimulus :type AI%20Stimulus%20Structure%20%28by%20ref%29))
  (if (Utilities|Struct|BreakAIStimulus Stimulus)
    (Utilities|Time|ClearandInvalidateTimerbyHandle (Variables|Default|GetLostSightHandle))
    (AI|Components|Blackboard|SetValueasObject (Variables|Default|GetBlackboard) (Variables|Default|GetTarget) Enemy)
    (else
      (bind _returnvalue (Utilities|Time|SetTimerbyEvent (delegate Custom|Lost%20Sight) (Variables|Default|GetLoseSightDuration)))
      (Variables|Default|SetLostSightHandle _returnvalue))))

(fn ConstructionScript)