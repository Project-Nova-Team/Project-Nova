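; BP_Monster is an AI-controlled monster that can lie in ambush.
; On BeginPlay it enters ambush mode at its current location when StartInAmbush is set.
; Enter Ambush Mode moves it to a given location and sets the Ambushing key on its AI controller's Blackboard, and Exit Ambush Mode clears that key.
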(event EventBeginPlay
  (if (Variables|AI|General|GetbStartInAmbush)
    (CallFunction|EnterAmbushMode (Transformation|GetActorLocation))))

(fn ConstructionScript)

(fn EnterAmbushMode
  (params (AmbushLocation :type Vector))
  (Transformation|SetActorLocation AmbushLocation false false)
  (AI|Components|Blackboard|SetValueasBool (AI|GetBlackboard (.AsAIController (Utilities|Casting|CastToAIController (Pawn|GetController)))) (Variables|Default|GetAmbushing) true))

(fn ExitAmbushMode
  (AI|Components|Blackboard|SetValueasBool (AI|GetBlackboard (.AsAIController (Utilities|Casting|CastToAIController (Pawn|GetController)))) (Variables|Default|GetAmbushing) false))