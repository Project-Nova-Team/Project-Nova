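; AI controller for testing patrol behavior on a PatrolTestAI pawn.
; On BeginPlay it runs the Patrol behavior tree and casts the controlled pawn to PatrolTestAI.
; If the Blackboard's display name is non-empty, it prints it and copies the pawn's Instruction object into the Instruction key; otherwise it prints a debug "None".
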(event EventBeginPlay
  (bind _blackboard (Variables|Default|GetBlackboard))
  (bind _returnvalue (Utilities|GetDisplayName _blackboard))
  (AI|RunBehaviorTree "/Game/AI/Patrol.Patrol")
  (bind _aspatrol_test_ai (Utilities|Casting|CastToPatrolTestAI (Pawn|GetControlledPawn)))
  (if (Utilities|Enum|Equal(Enum) _returnvalue "")
    (Development|PrintString "None")
    (else
      (Development|PrintString _returnvalue)
      (AI|Components|Blackboard|SetValueasObject _blackboard (Variables|Default|GetInstruction) (Variables|/Script/UnrealPlayground.AIBase|GetInstruction _aspatrol_test_ai)))))

(fn ConstructionScript)