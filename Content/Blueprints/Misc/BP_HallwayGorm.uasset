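; BP_HallwayGorm is a zombie-animated Gorm that reacts to the results of quick-time event actions.
; A successful result plays a headbutt, attack or neck-bite montage chosen by success count.
; An unsuccessful result plays damage sound and hit montage, or, if the event is completed, death sound and sets Dead.
; StartQuickTime and the post-montage completion branch are empty, and the collision and movement shutdown is unconnected.
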(event Custom|StartQuickTime)

(event EventQuickTimeActionComplete
  (params (bSucceeded :type Boolean) (bCompleted :type Boolean) (SuccessCount :type Integer))
  (bind _returnvalue (Transformation|GetActorLocation))
  (if bSucceeded
    (Animation|Montage|PlayMontage (Variables|Character|GetMesh) (Utilities|Select :Index (- SuccessCount 1) :Option%200 "/Game/Animation/Zombie/AM_Zombie_HeadButt.AM_Zombie_HeadButt" :Option%201 "/Game/Animation/Zombie/AttackMontage.AttackMontage" :Option%202 "/Game/Animation/Zombie/AM_Zombie_NeckBite.AM_Zombie_NeckBite")
      (:OnCompleted
        _))
    (elif bCompleted
      (Audio|PlaySoundatLocation "/Game/Audio/SFX/Gorm/SFX_Gorm_Death.SFX_Gorm_Death" _returnvalue "0, 0, 0" 1.0 1.0 0.0 0 0 0)
      (Variables|Default|SetbDead true)
      (else
        (Audio|PlaySoundatLocation "/Game/Audio/SFX/Gorm/SFX_Gorm_DamageTaken.SFX_Gorm_DamageTaken" _returnvalue "0, 0, 0" 1.0 1.0 0.0 0 0 0)
        (Animation|Montage|PlayMontage (Variables|Character|GetMesh) "/Game/Animation/Zombie/AM_Zombie_Hit.AM_Zombie_Hit"
          (:OnCompleted
            _)))))
  (if bCompleted
    _))

(fn ConstructionScript)