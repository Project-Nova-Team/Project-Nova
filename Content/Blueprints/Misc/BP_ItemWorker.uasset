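; BP_ItemWorker is a worker Blueprint that holds a configurable item at its mesh's Weapon_Socket.
; On BeginPlay it runs the parent logic, then sets the Item child actor component's class from ItemClass.
; It attaches the spawned child actor to the socket, keeping world scale, and applies LocationOffset and RotationOffset as relative adjustments.
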(event EventBeginPlay
  (bind _item (Variables|Default|GetItem))
  (bind _childactor (Variables|/Script/Engine.ChildActorComponent|GetChildActor _item))
  (|CallParentFunction)
  (ChildActorComponent|SetChildActorClass _item (Variables|Default|GetItemClass))
  (Transformation|AttachComponentToComponent _childactor (Variables|Character|GetMesh) "Weapon_Socket" "KeepRelative" "KeepRelative" "KeepWorld" false)
  (Transformation|SetActorRelativeLocation _childactor (Variables|Default|GetLocationOffset))
  (Transformation|SetActorRelativeRotation _childactor (Variables|Default|GetRotationOffset)))

(fn ConstructionScript)