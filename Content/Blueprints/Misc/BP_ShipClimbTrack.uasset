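; BP_ShipClimbTrack is a scripted track that moves the player along a spline, apparently a climb on the ship.
; InitiateMove turns on Tick, which first turns the player's camera anchor at a constant rate to a target look rotation.
; It then moves the player along the spline over MoveTime.
; At the end it stops ticking, sets the player's state to Walking and has them pick up the RealWrench weapon.
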(event Custom|Initiate%20Move
  (Actor|Tick|SetActorTickEnabled true))

(event EventTick
  (params (DeltaSeconds :type Float%20%28single-precision%29))
  (bind _player (Variables|Default|GetPlayer))
  (bind _targetlook (Variables|Default|GetTargetLook))
  (bind _cameraanchor (Variables|/Script/ProjectNova.Shooter|GetCameraAnchor _player))
  (bind _relativerotation (Variables|/Script/Engine.SceneComponent|GetRelativeRotation _cameraanchor))
  (bind _returnvalue (Class|KismetMathLibrary|RInterptoConstant _relativerotation _targetlook DeltaSeconds 9e+01))
  (if (Variables|Default|GetRotationComplete)
    (bind _output_get (Variables|Default|SetTimer (+ DeltaSeconds (Variables|Default|GetTimer))))
    (Transformation|SetActorLocation (Variables|Default|GetPlayer) (Spline|GetLocationatTime (Variables|Default|GetSpline) (Math|Float|Clamp(Float) (/ _output_get (Variables|Default|GetMoveTime))) "World" false) false false)
    (if (== (Math|Float|Clamp(Float) (/ _output_get (Variables|Default|GetMoveTime))) 1.0)
      (Actor|Tick|SetActorTickEnabled false)
      (Class|Shooter|SetStateOverride (Variables|Default|GetPlayer) "Walking")
      (Class|CombatComponent|PickUpWeapon (Variables|/Script/ProjectNova.Shooter|GetCombat (Variables|Default|GetPlayer)) (Variables|Default|GetRealWrench)))
    (else
      (Transformation|SetRelativeRotation _cameraanchor _returnvalue false false)
      (if (Math|Rotator|Equal(Rotator) _returnvalue _targetlook 0.0001)
        (Variables|Default|SetRotationComplete true)))))

(fn ConstructionScript)