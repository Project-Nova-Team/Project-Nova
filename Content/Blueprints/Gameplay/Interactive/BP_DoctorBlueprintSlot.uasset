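; BP_DoctorBlueprintSlot is a one-time interactable slot where the doctor's blueprints are placed, advancing progression in the level.
; On BlueprintInteract it reveals the Blueprints component, turns off further interaction and disables the mesh's collision.
; The same event unlocks the entrance and elevator doors and activates the linked elevator and dialogue triggers.
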(event EventBlueprintInteract
  (params (EventSender :type Pawn%20Object%20Reference))
  (Variables|/Script/UnrealPlayground.Door|SetbIsLocked (Variables|Default|GetDoor_Entrance) false)
  (Rendering|SetVisibility (Variables|Default|GetBlueprints) true false)
  (Variables|Default|SetbCanInteract false)
  (Collision|SetCollisionEnabled (Variables|Character|GetMesh) "NoCollision")
  (Variables|/Script/UnrealPlayground.Door|SetbIsLocked (Variables|Default|GetElevatorDoor) false)
  (Class|Trigger|SetActive (Variables|Default|GetElevatorTrigger) true)
  (Class|Trigger|SetActive (Variables|Default|GetDialogue%20Trigger) true))

(fn ConstructionScript)