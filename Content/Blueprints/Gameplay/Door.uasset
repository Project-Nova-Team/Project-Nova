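; Door actor that shows its lock state through the emissive color of its frame.
; The construction script creates a dynamic material instance on the first material slot of the Frame component.
; On BeginPlay it binds to the OnDoorLockStatusChange dispatcher, whose handler switches the EmissiveColor parameter between the locked and opened colors.
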(event Custom|Lock%20Status%20Changed
  (params (bJustLocked :type Boolean))
  (bind _dynmaterial (Variables|Default|GetDynMaterial))
  (if bJustLocked
    (Rendering|Material|SetVectorParameterValue _dynmaterial "EmissiveColor" (Variables|Default|GetLockedColor) :!class /Script/Engine.MaterialInstanceDynamic)
    (else
      (Rendering|Material|SetVectorParameterValue _dynmaterial "EmissiveColor" (Variables|Default|GetOpenedColor) :!class /Script/Engine.MaterialInstanceDynamic))))

(event EventBeginPlay
  (EventDispatchers|AssignOnDoorLockStatusChange (delegate Custom|Lock%20Status%20Changed)))

(fn ConstructionScript
  (bind _returnvalue (Rendering|Material|CreateDynamicMaterialInstance (Variables|Default|GetFrame) 0 0 "None" :!class /Script/Engine.PrimitiveComponent))
  (Variables|Default|SetDynMaterial _returnvalue))