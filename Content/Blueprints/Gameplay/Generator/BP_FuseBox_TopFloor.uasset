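; BP_FuseBox_TopFloor is the top-floor fuse box interactable that restores light and unlocks a door when fixed.
; It extends a parent fuse box Blueprint by calling the parent interact event, then adding its own results.
; Interaction clears the lock on the referenced DoorLock, plays a metallic wrench impact at the box and raises the referenced LightOn point light's intensity.
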(event EventBeginPlay
  (|CallParentFunction) ; This node is disabled and will not be called.\nDrag off pins to build functionality.
)

(event EventBlueprintInteract
  (params (EventSender :type Pawn%20Object%20Reference))
  ;[1 1 1] Attach whatever you want to happen after you fix the fuse box here!
  (|CallParentFunction EventSender)
  (Variables|/Script/ProjectNova.Door|SetbIsLocked (Variables|Default|GetDoorLock) false)
  (Audio|PlaySoundatLocation "/Game/Audio/SFX/Weapon/Wrench/SFX_Wrench_ImpactMetal.SFX_Wrench_ImpactMetal" (Transformation|GetActorLocation) "0, 0, 0" 1.0 1.0 0.0 0 0 0)
  (Rendering|Components|Light|SetIntensity (Variables|/Game/Blueprints/Lights/BP_PoolLight.BP_PoolLight_C|GetPointLight (Variables|Default|GetLightOn)) 8.0))

(fn ConstructionScript
  (|CallParentFunction))