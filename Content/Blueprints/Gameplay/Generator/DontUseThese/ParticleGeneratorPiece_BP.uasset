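; Generator piece Blueprint that plays intermittent particle and audio effects until the piece is repaired.
; From BeginPlay, a self-recalling Play event runs both effects for a fixed burst, pauses for a short random interval, then repeats while unrepaired.
; The OnGeneratorPieceRepair dispatcher sets the repaired flag, stops the audio and deactivates the particles, which ends the loop.
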(event Custom|PieceRepaired
  (Variables|Default|SetbIsRepaired true)
  (Audio|Components|Audio|Stop (Variables|Default|GetAudio))
  (Components|Activation|Deactivate (Variables|Default|GetParticleSystem)))

(event Custom|Play
  (bind _audio (Variables|Default|GetAudio))
  (bind _particlesystem (Variables|Default|GetParticleSystem))
  (Audio|Components|Audio|Play _audio 0.0)
  (Components|Activation|Activate _particlesystem true)
  (Utilities|FlowControl|Delay 4.0)
  (Components|Activation|Deactivate _particlesystem)
  (Audio|Components|Audio|Stop _audio)
  (Utilities|FlowControl|Delay (Math|Random|RandomFloatinRange 2.0 3.0))
  (if (not (Variables|Default|GetbIsRepaired))
    (CallFunction|Play)))

(event EventBeginPlay
  (CallFunction|Play)
  (EventDispatchers|AssignOnGeneratorPieceRepair (delegate Custom|PieceRepaired)))

(fn ConstructionScript)