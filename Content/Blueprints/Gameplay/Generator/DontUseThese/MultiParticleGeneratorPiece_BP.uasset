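; Generator piece with two particle systems and audio that signal damage until it is repaired.
; On begin play it starts a burst loop that plays effects and sound for a few seconds, stops them, waits a short random interval, then repeats.
; The piece's repair event sets a flag that ends the loop and immediately stops the audio and both particle systems.
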(event Custom|Repaired
  (Variables|Default|SetbIsRepaired true)
  (Audio|Components|Audio|Stop (Variables|Default|GetAudio))
  (Components|Activation|Deactivate (Variables|Default|GetParticleSystem))
  (Components|Activation|Deactivate (Variables|Default|GetParticleSystemTwo)))

(event Custom|ParticlePlay
  (bind _particlesystemtwo (Variables|Default|GetParticleSystemTwo))
  (bind _audio (Variables|Default|GetAudio))
  (bind _particlesystem (Variables|Default|GetParticleSystem))
  (Audio|Components|Audio|Play _audio 0.0)
  (Components|Activation|Activate _particlesystem true)
  (Components|Activation|Activate _particlesystemtwo true)
  (Utilities|FlowControl|Delay 4.0)
  (Components|Activation|Deactivate _particlesystem)
  (Components|Activation|Deactivate _particlesystemtwo)
  (Audio|Components|Audio|Stop _audio)
  (Utilities|FlowControl|Delay (Math|Random|RandomFloatinRange 2.0 3.0))
  (if (not (Variables|Default|GetbIsRepaired))
    (CallFunction|ParticlePlay)))

(event EventBeginPlay
  (CallFunction|ParticlePlay)
  (EventDispatchers|AssignOnGeneratorPieceRepair (delegate Custom|Repaired)))

(fn ConstructionScript
  (|CallParentFunction))