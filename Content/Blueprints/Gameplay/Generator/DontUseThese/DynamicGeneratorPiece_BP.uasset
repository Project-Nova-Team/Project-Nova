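; Generator piece actor whose lightbulb flickers with a malfunction sound until the piece is repaired.
; On BeginPlay it creates a dynamic material for mesh slot 1 and binds to the flicker and repair events.
; Each flicker toggles the Glow texture parameter between enabled and disabled emission maps.
; Repair stops the flickering and leaves the enabled glow texture showing.
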(event Custom|Piece%20Repaired
  ;[1 1 1] When repaired, we stop flickering the materials
  (Class|DynamicGeneratorPiece|StopFlicker)
  (Rendering|Material|SetTextureParameterValue (Variables|Default|GetDynMaterial) "Glow" (Variables|Default|GetEnabledTexture)))

(event Custom|Flicker
  (bind _dynmaterial (Variables|Default|GetDynMaterial))
  ;[1 1 1] Just periodically switches between two emission maps which will turn one bulb on/off
  (Audio|PlaySoundatLocation "/Game/Audio/SFX/Misc/Generator/SFX_MISC_GEN_LightbulbMalfunction.SFX_MISC_GEN_LightbulbMalfunction" (Transformation|GetActorLocation) "0, 0, 0" 0.3 1.0 0.0 "/Game/Audio/SFX/Weapon/BulletImpact.BulletImpact" "/Game/Audio/SFX/PlayOldest.PlayOldest" self)
  (bind _output_get (Variables|Default|SetbIsFlickeredOn (not (Variables|Default|GetbIsFlickeredOn))))
  (if _output_get
    (Rendering|Material|SetTextureParameterValue _dynmaterial "Glow" (Variables|Default|GetEnabledTexture))
    (else
      (Rendering|Material|SetTextureParameterValue _dynmaterial "Glow" (Variables|Default|GetDisabledTexture)))))

(event EventBeginPlay
  (bind _mesh (Variables|Character|GetMesh))
  (bind _returnvalue (Rendering|Material|CreateDynamicMaterialInstance _mesh 1 0 "None" :!class /Script/Engine.PrimitiveComponent))
  (bind _output_get (Variables|Default|SetDynMaterial _returnvalue))
  (Rendering|Material|SetMaterial _mesh 1 _output_get)
  (EventDispatchers|AssignOnGeneratorPieceRepair (delegate Custom|Piece%20Repaired))
  (EventDispatchers|AssignOnFlicker (delegate Custom|Flicker)))

(fn ConstructionScript)