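; Base generator that shows repair progress on its screen and powers up when interacted with.
; On BeginPlay it gathers its particle, interactable and dynamic child-actor pieces into an array and binds to the piece-repaired event.
; Each repair swaps the screen texture on a dynamic material by repaired count.
; Interacting shows the last screen texture, plays completion and power-up sounds, then starts the audio component after a long delay.
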(event Custom|Piece%20Repaired
  (params (RepairedPieceCount :type Integer))
  (Rendering|Material|SetTextureParameterValue (Variables|Default|GetDynMaterial) "DiffuseTexture" (Utilities|Array|Get(acopy) (Variables|Default|GetScreenTextures) RepairedPieceCount)))

(event EventBeginPlay
  (bind _mesh (Variables|Character|GetMesh))
  (bind _returnvalue (Rendering|Material|CreateDynamicMaterialInstance _mesh 0 0 "None" :!class /Script/Engine.PrimitiveComponent))
  (bind _output_get (Variables|Default|SetDynMaterial _returnvalue))
  (Rendering|Material|SetMaterial _mesh 0 _output_get)
  (bind _asparticle_generator_piece_bp (Utilities|Casting|CastToParticleGeneratorPiece_BP (Variables|/Script/Engine.ChildActorComponent|GetChildActor (Variables|Default|GetPieceOne))))
  (bind _asinteractable_generator_piece_bp (Utilities|Casting|CastToInteractableGeneratorPiece_BP (Variables|/Script/Engine.ChildActorComponent|GetChildActor (Variables|Default|GetPieceTwo))))
  (bind _asdynamic_generator_piece_bp (Utilities|Casting|CastToDynamicGeneratorPiece_BP (Variables|/Script/Engine.ChildActorComponent|GetChildActor (Variables|Default|GetPieceThree))))
  (Variables|Default|SetPieces (Utilities|Array|MakeArray _asdynamic_generator_piece_bp _asinteractable_generator_piece_bp _asparticle_generator_piece_bp))
  (EventDispatchers|AssignOnPieceRepaired (delegate Custom|Piece%20Repaired)))

(event EventBlueprintInteract
  (params (EventSender :type Pawn%20Object%20Reference))
  (bind _returnvalue (Transformation|GetActorLocation))
  (bind _screentextures (Variables|Default|GetScreenTextures))
  (Rendering|Material|SetTextureParameterValue (Variables|Default|GetDynMaterial) "DiffuseTexture" (Utilities|Array|Get(acopy) _screentextures (- (Utilities|Array|Length _screentextures) 1)))
  (Audio|PlaySoundatLocation "/Game/Audio/SFX/Misc/Generator/SFX_MISC_GEN_TaskCompleted.SFX_MISC_GEN_TaskCompleted" _returnvalue "0, 0, 0" 1.0 1.0 0.0 0 0 0)
  (Utilities|FlowControl|Delay 0.2)
  (Audio|PlaySoundatLocation "/Game/Audio/SFX/Misc/Generator/SFX_MISC_GEN_PowerUp.SFX_MISC_GEN_PowerUp" _returnvalue "0, 0, 0" 1.0 1.0 0.0 0 0 0)
  (Utilities|FlowControl|Delay 33.604)
  (Audio|Components|Audio|Play (Variables|Default|GetAudio) 0.0))

(fn ConstructionScript)