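; Interactable generator Blueprint that changes a set of linked level actors when the player or another sender interacts with it.
; On interact, after the parent logic, it locks one door, unlocks two others and makes a vent's health invincible.
; It also recolors referenced point and rect lights to pale blue.
; The Spotlight and Pointlight3 recolors are disconnected because those references were unset.
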(event EventBeginPlay
  (|CallParentFunction) ; This node is disabled and will not be called.\nDrag off pins to build functionality.
)

(event EventBlueprintInteract
  (params (EventSender :type Pawn%20Object%20Reference))
  (|CallParentFunction EventSender)
  (Class|Door|SetIsLocked (Variables|Default|GetDoorLock) true)
  (Variables|/Script/ProjectNova.HealthComponent|SetbIsInvincible (Variables|/Script/ProjectNova.Vent|GetHealth (Variables|Default|GetVent)) true)
  (Class|Door|SetIsLocked (Variables|Default|GetDoorUnlock1) false)
  (Class|Door|SetIsLocked (Variables|Default|GetDoorUnlock2) false)
  (Rendering|Components|Light|SetLightColor (Variables|/Script/Engine.PointLight|GetPointLightComponent (Variables|Default|GetPointlight1)) "(R=0.392701,G=0.388869,B=1.000000,A=1.000000)" true)
  (Rendering|Components|Light|SetLightColor (Variables|/Script/Engine.PointLight|GetPointLightComponent (Variables|Default|GetPointlight2)) "(R=0.392701,G=0.388869,B=1.000000,A=1.000000)" true)
  (Rendering|Components|Light|SetLightColor (Variables|/Script/Engine.PointLight|GetPointLightComponent (Variables|Default|GetPointlight4)) "(R=0.392701,G=0.388869,B=1.000000,A=1.000000)" true)
  (Rendering|Components|Light|SetLightColor (Variables|/Script/Engine.RectLight|GetRectLightComponent (Variables|Default|GetRectlight1)) "(R=0.392701,G=0.388869,B=1.000000,A=1.000000)" true)
  (Rendering|Components|Light|SetLightColor (Variables|/Script/Engine.RectLight|GetRectLightComponent (Variables|Default|GetRectlight2)) "(R=0.392701,G=0.388869,B=1.000000,A=1.000000)" true)
  (Rendering|Components|Light|SetLightColor (Variables|/Script/Engine.RectLight|GetRectLightComponent (Variables|Default|GetRectlight3)) "(R=0.392701,G=0.388869,B=1.000000,A=1.000000)" true))

(fn ConstructionScript
  (|CallParentFunction))