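; BP_Generator2 is an interactable generator that changes the lighting of its surroundings when used.
; On BlueprintInteract it calls the parent logic, then tints eight referenced rect lights and four point lights a soft blue.
; It also switches on three of those point lights; the fourth, named as already on, only changes color.
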(event EventBlueprintInteract
  (params (EventSender :type Pawn%20Object%20Reference))
  (bind _pointlight2 (Variables|Default|GetPointlight2))
  (bind _pointlight3 (Variables|Default|GetPointlight3))
  (bind _pointlight1 (Variables|Default|GetPointlight1))
  (|CallParentFunction EventSender)
  (Rendering|Components|Light|SetLightColor (Variables|/Script/Engine.RectLight|GetRectLightComponent (Variables|Default|GetRectlight1)) "(R=0.392701,G=0.388869,B=1.000000,A=1.000000)" true)
  (Rendering|Components|Light|SetLightColor (Variables|/Script/Engine.RectLight|GetRectLightComponent (Variables|Default|GetRectlight2)) "(R=0.392701,G=0.388869,B=1.000000,A=1.000000)" true)
  (Rendering|Components|Light|SetLightColor (Variables|/Script/Engine.RectLight|GetRectLightComponent (Variables|Default|GetRectlight3)) "(R=0.392701,G=0.388869,B=1.000000,A=1.000000)" true)
  (Rendering|Components|Light|SetLightColor (Variables|/Script/Engine.RectLight|GetRectLightComponent (Variables|Default|GetRectlight4)) "(R=0.392701,G=0.388869,B=1.000000,A=1.000000)" true)
  (Rendering|Components|Light|SetLightColor (Variables|/Script/Engine.RectLight|GetRectLightComponent (Variables|Default|GetRectlight5)) "(R=0.392701,G=0.388869,B=1.000000,A=1.000000)" true)
  (Rendering|Components|Light|SetLightColor (Variables|/Script/Engine.RectLight|GetRectLightComponent (Variables|Default|GetRectlight6)) "(R=0.392701,G=0.388869,B=1.000000,A=1.000000)" true)
  (Rendering|Components|Light|SetLightColor (Variables|/Script/Engine.RectLight|GetRectLightComponent (Variables|Default|GetRectlight7)) "(R=0.392701,G=0.388869,B=1.000000,A=1.000000)" true)
  (Rendering|Components|Light|SetLightColor (Variables|/Script/Engine.RectLight|GetRectLightComponent (Variables|Default|GetRectlight8)) "(R=0.392701,G=0.388869,B=1.000000,A=1.000000)" true)
  (Rendering|Components|Light|SetLightColor (Variables|/Script/Engine.PointLight|GetPointLightComponent _pointlight1) "(R=0.392701,G=0.388869,B=1.000000,A=1.000000)" true)
  (Rendering|SetVisibility (Variables|/Script/Engine.PointLight|GetPointLightComponent _pointlight1) true false)
  (Rendering|Components|Light|SetLightColor (Variables|/Script/Engine.PointLight|GetPointLightComponent _pointlight2) "(R=0.392701,G=0.388869,B=1.000000,A=1.000000)" true)
  (Rendering|SetVisibility (Variables|/Script/Engine.PointLight|GetPointLightComponent _pointlight2) true false)
  (Rendering|Components|Light|SetLightColor (Variables|/Script/Engine.PointLight|GetPointLightComponent _pointlight3) "(R=0.392701,G=0.388869,B=1.000000,A=1.000000)" true)
  (Rendering|SetVisibility (Variables|/Script/Engine.PointLight|GetPointLightComponent _pointlight3) true false)
  (Rendering|Components|Light|SetLightColor (Variables|/Script/Engine.PointLight|GetPointLightComponent (Variables|Default|GetPointlight4_AlreadyOn)) "(R=0.392701,G=0.388869,B=1.000000,A=1.000000)" true))

(fn ConstructionScript
  (|CallParentFunction))