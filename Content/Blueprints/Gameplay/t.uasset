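; Debug test actor that visualizes the start and end tangents of its Spline component.
; BeginPlay prints the world-space tangents at spline times 0 and 1 to the screen.
; Tick redraws both tangents every frame as colored debug lines from the actor's location, rather than from the spline points themselves.
; The construction script is empty.
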(event EventBeginPlay
  (Development|PrintString (Utilities|String|ToString(Vector) (Class|SplineComponent|GetTangentatTime (Variables|Default|GetSpline) 0.0 "World" false)) true true "(R=0.000000,G=0.660000,B=1.000000,A=1.000000)" 1e+01)
  (Development|PrintString (Utilities|String|ToString(Vector) (Class|SplineComponent|GetTangentatTime (Variables|Default|GetSpline) 1.0 "World" false)) true true "(R=1.000000,G=0.000000,B=0.787745,A=1.000000)" 1e+01))

(event EventTick
  (params (DeltaSeconds :type Float%20%28single-precision%29))
  (bind _returnvalue (Transformation|GetActorLocation))
  (Rendering|Debug|DrawDebugLine _returnvalue (+ _returnvalue (Class|SplineComponent|GetTangentatTime (Variables|Default|GetSpline) 0.0 "World" false)) "(R=0.000000,G=0.391990,B=1.000000,A=1.000000)" 0.02 1.0)
  (Rendering|Debug|DrawDebugLine _returnvalue (+ (Class|SplineComponent|GetTangentatTime (Variables|Default|GetSpline) 1.0 "World" false) _returnvalue) "(R=1.000000,G=0.000000,B=0.880255,A=1.000000)" 0.02 1.0))

(fn ConstructionScript)