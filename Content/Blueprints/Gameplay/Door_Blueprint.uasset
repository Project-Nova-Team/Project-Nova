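; Door actor Blueprint that plays open and close sounds and shows its lock status through the color of its frame.
; The construction script creates a dynamic material instance from the Door material and applies it to the Frame.
; Door open and close events play their sounds at the actor location, while lock status changes switch the material's EmissiveColor between locked and open colors.
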(event EventDoorClose
  (Audio|PlaySoundatLocation "/Game/Audio/SFX/Misc/DoorClose.DoorClose" (Transformation|GetActorLocation) "0, 0, 0" 1.0 1.0 0.0 "/Game/Audio/SFX/Weapon/BulletImpact.BulletImpact" 0 0))

(event EventDoorOpen
  (Audio|PlaySoundatLocation "/Game/Audio/SFX/Misc/DoorOpen.DoorOpen" (Transformation|GetActorLocation) "0, 0, 0" 1.0 1.0 0.0 "/Game/Audio/SFX/Weapon/BulletImpact.BulletImpact" 0 0))

(event EventLockStatusChange
  (params (LockStatus :type Boolean))
  (Rendering|Material|SetVectorParameterValue (Variables|Default|GetDynamicMat) "EmissiveColor" (select LockStatus (Variables|Default|GetLockedColor) (Variables|Default|GetOpenColor)) :!class /Script/Engine.MaterialInstanceDynamic))

(fn ConstructionScript
  (bind _returnvalue (Rendering|Material|CreateDynamicMaterialInstance (Variables|Default|GetFrame) 0 "/Game/Art/Materials/Door.Door" "None" :!class /Script/Engine.PrimitiveComponent))
  (bind _output_get (Variables|Default|SetDynamicMat _returnvalue))
  (Rendering|Material|SetMaterial (Variables|Default|GetFrame) 0 _output_get))