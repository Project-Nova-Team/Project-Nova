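; BP_Vent handles the sound feedback for a vent as it is enabled and disabled.
; BeginPlay binds handlers to the OnVentEnabled and OnVentDisabled dispatchers.
; Enabling plays an activation sound at the actor's location, then starts the Audio component after a delay matching that clip's duration.
; Disabling stops the Audio component and plays a deactivation sound, without cancelling any pending delayed start.
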(event Custom|VentEnabled
  (Audio|PlaySoundatLocation "/Game/Audio/SFX/Vent/SFX_Vent_Activate.SFX_Vent_Activate" (Transformation|GetActorLocation) "0, 0, 0" 1.0 1.0 0.0 0 0 0)
  (Utilities|FlowControl|Delay (Variables|/Script/Engine.SoundBase|GetDuration (stale EventBeginPlay _output_get)))
  (Audio|Components|Audio|Play (Variables|Default|GetAudio) 0.0))

(event Custom|VentDisabled
  (Audio|Components|Audio|Stop (Variables|Default|GetAudio))
  (Audio|PlaySoundatLocation "/Game/Audio/SFX/Vent/SFX_Vent_Deactivate.SFX_Vent_Deactivate" (Transformation|GetActorLocation) "0, 0, 0" 1.0 1.0 0.0 0 0 0))

(event EventBeginPlay
  (bind _output_get (Variables|Default|SetEnableClip "/Game/Audio/SFX/Vent/SFX_Vent_Activate.SFX_Vent_Activate"))
  (EventDispatchers|AssignOnVentEnabled (delegate Custom|VentEnabled))
  (EventDispatchers|AssignOnVentDisabled (delegate Custom|VentDisabled)))

(fn ConstructionScript)