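; BP_PromptTrigger is a trigger that shows an interaction prompt on the HUD of the Shooter that activates it.
; On activation it caches the Shooter, sets IsPrompted, and passes configurable prefix text, key texture and suffix text to the ShooterHUD found through the controller.
; On exit it hides the prompt through the cached HUD and clears the flag, without checking who exited.
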(event EventTriggerActivated
  (params (Activator :type Pawn%20Object%20Reference))
  (bind _asshooter (Utilities|Casting|CastToShooter Activator))
  (bind _output_get (Variables|Default|SetShooter _asshooter))
  (Variables|/Script/UnrealPlayground.Shooter|SetbIsPrompted _output_get true)
  (CallFunction|ShowShooterUI))

(event EventTriggerExited
  (params (Activator :type Pawn%20Object%20Reference))
  (CallFunction|HideShooterUI)
  (Variables|/Script/UnrealPlayground.Shooter|SetbIsPrompted (Variables|Default|GetShooter) false))

(fn ConstructionScript)

(fn ShowShooterUI
  (bind _asshooter_controller (Utilities|Casting|CastToShooterController (Pawn|GetController (Variables|Default|GetShooter))))
  (bind _asshooter_hud (Utilities|Casting|CastToShooterHUD (HUD|GetHUD _asshooter_controller)))
  (bind _output_get (Variables|Default|SetShooterHUD _asshooter_hud))
  (Class|ShooterHUD|ShowInteractionPrompt _output_get (Utilities|Struct|MakeInteractionPrompt (Variables|Default|GetPrefixText) (Variables|Default|GetKeyTexture) (Variables|Default|GetSuffixText) "")))

(fn HideShooterUI
  (Class|ShooterHUD|HideInteractionPrompt (Variables|Default|GetShooterHUD) (Utilities|Struct|MakeInteractionPrompt "Press" 0 "to pick up " "object.")))