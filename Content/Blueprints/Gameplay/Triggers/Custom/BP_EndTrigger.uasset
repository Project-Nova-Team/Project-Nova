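; BP_EndTrigger is a custom trigger that runs the game's ending sequence when activated.
; It clears the player's objective, closes and locks a door, and plays a sound to completion.
; It then starts an elevator during a slow fade to black with audio.
; Finally it stops the elevator, hides the weapon HUD, shows the WBP_Ending widget, and loads the title screen after timed delays.
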(event EventTriggerActivated
  (params (Activator :type Pawn%20Object%20Reference))
  (bind _door (Variables|Default|GetDoor))
  (bind _sound (Variables|Default|GetSound))
  (bind _player (Variables|Default|GetPlayer))
  (bind _returnvalue (Pawn|GetController _player))
  (bind _asshooter_controller (Utilities|Casting|CastToShooterController _returnvalue))
  (Class|Shooter|ClearObjective (Variables|Default|GetPlayer))
  (Class|Door|CloseDoor _door false)
  (Variables|/Script/ProjectNova.Door|SetbIsLocked _door true)
  (Audio|PlaySound2D _sound 1.0 1.0 0.0 0 0)
  (Utilities|FlowControl|Delay (Variables|/Script/Engine.SoundBase|GetDuration _sound))
  (Class|Elevator|StartElevator (Variables|Default|GetElevator))
  (CameraFades|StartCameraFade :self (Variables|/Script/Engine.PlayerController|GetPlayerCameraManager _asshooter_controller) :FromAlpha 0.0 :ToAlpha 1.0 :Duration 1e+01 :bShouldFadeAudio true :bHoldWhenFinished true)
  (Utilities|FlowControl|Delay 11.0)
  (Class|Elevator|StopElevator (Variables|Default|GetElevator))
  (Widget|SetVisibility (Variables|/Script/ProjectNova.ShooterHUD|GetWeaponDisplayWidget (Variables|/Script/ProjectNova.ShooterController|GetShooterHUD _asshooter_controller)) "Collapsed")
  (bind _returnvalue_2 (UserInterface|CreateWidget "/Game/Blueprints/UI/Widgets/WBP_Ending.WBP_Ending_C" _asshooter_controller))
  (UserInterface|Viewport|AddtoViewport _returnvalue_2 0)
  (Utilities|FlowControl|Delay 1e+01)
  (Game|OpenLevel(byName) "TitleScreen"))

(fn ConstructionScript
  (|CallParentFunction))