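; BP_DocDialoge is a scripted trigger that stages the Doc dialogue scene and moves the player's objective on.
; On activation it unlocks the data room, activates DocTrigger, locks the lab and Doc room doors, clears the objective and plays a level sequence.
; A fixed delay of about a minute, rather than a sequence-finished callback, then gates the new objective to meet Engi-26 and unlocks both doors.
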(event EventTriggerActivated
  (params (Activator :type Pawn%20Object%20Reference))
  (Variables|/Script/ProjectNova.Door|SetbIsLocked (Variables|Default|GetDataRoom) false)
  (Variables|/Script/ProjectNova.Trigger|SetbIsActive (Variables|Default|GetDocTrigger) true)
  (Variables|/Script/ProjectNova.Door|SetbIsLocked (Variables|Default|GetLabDoor) true)
  (Variables|/Script/ProjectNova.Door|SetbIsLocked (Variables|Default|GetDocRoom) true)
  (Class|Shooter|ClearObjective (Variables|Default|GetPlayer))
  (bind _returnvalue (Sequencer|Player|CreateLevelSequencePlayer (Variables|Default|GetSequence)))
  (Sequencer|Player|Play _returnvalue :!class /Script/MovieScene.MovieSceneSequencePlayer)
  (Utilities|FlowControl|Delay 62.299999)
  (Class|Shooter|StartNewObjective (Variables|Default|GetPlayer) (Utilities|Struct|MakeObjective "Meet back with Engi-26" false "WAYPOINT_Static" 0 0 1e+02 1e+02))
  (Variables|/Script/ProjectNova.Door|SetbIsLocked (Variables|Default|GetDocRoom) false)
  (Variables|/Script/ProjectNova.Door|SetbIsLocked (Variables|Default|GetLabDoor) false))

(fn ConstructionScript
  (|CallParentFunction))