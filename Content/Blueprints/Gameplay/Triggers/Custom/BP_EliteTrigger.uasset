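; BP_EliteTrigger is a custom trigger that starts an elite encounter with a Monster and three Gorms, setting an escape objective for the activating Shooter.
; On BeginPlay it waits briefly, then enables query and physics collision on the four creatures' capsules.
; On activation it plays the Predator intro sound, marks all four as loaded, then starts the music loop after a fixed delay plus the intro's duration.
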(event EventBeginPlay
  (Utilities|FlowControl|Delay 0.02)
  (Collision|SetCollisionEnabled (Variables|/Script/Engine.Character|GetCapsuleComponent (Variables|Default|GetMonster)) "QueryAndPhysics"))

(event EventTriggerActivated
  (params (Activator :type Pawn%20Object%20Reference))
  (bind _predatorintro (Variables|Default|GetPredatorIntro))
  (Class|Shooter|StartNewObjective (.AsShooter (Utilities|Casting|CastToShooter Activator)) (Utilities|Struct|MakeObjective "Escape!" true "WAYPOINT_Static" 0 0 1e+02 1e+02))
  (Audio|PlaySound2D _predatorintro 1.0 1.0 0.0 0 0)
  (Variables|/Script/ProjectNova.BaseAI|SetbIsLoaded (Variables|Default|GetMonster) true)
  (Variables|/Script/ProjectNova.BaseAI|SetbIsLoaded (Variables|Default|GetGorm1) true)
  (Variables|/Script/ProjectNova.BaseAI|SetbIsLoaded (Variables|Default|GetGorm2) true)
  (Variables|/Script/ProjectNova.BaseAI|SetbIsLoaded (Variables|Default|GetGorm3) true)
  (Utilities|FlowControl|Delay 2.0)
  (Utilities|FlowControl|Delay (Variables|/Script/Engine.SoundBase|GetDuration _predatorintro))
  (Audio|PlaySound2D "/Game/Audio/Music/MUS_Predator_Loop.MUS_Predator_Loop" 1.0 1.0 0.0 0 0))

(fn ConstructionScript
  (|CallParentFunction))