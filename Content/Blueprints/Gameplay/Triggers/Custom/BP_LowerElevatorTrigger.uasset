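; BP_LowerElevatorTrigger is a level trigger that runs the lower elevator arrival sequence.
; On BeginPlay it fades the player camera in from black and starts the elevator after a short delay.
; When activated, it stops the elevator, opens the door, plays a power-down sound and gives the player the objective to find Engi-26.
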(event EventBeginPlay
  (CameraFades|StartCameraFade :self (Variables|/Script/Engine.PlayerController|GetPlayerCameraManager (.AsPlayer%20Controller (Utilities|Casting|CastToPlayerController (Pawn|GetController (Variables|Default|GetShooter))))) :FromAlpha 1.0 :Duration 6.0)
  (Utilities|FlowControl|Delay 0.2)
  (Class|Elevator|StartElevator (Variables|Default|GetElevator)))

(event EventTriggerActivated
  (params (Activator :type Pawn%20Object%20Reference))
  (Class|Elevator|StopElevator (Variables|Default|GetElevator))
  (Class|Door|OpenDoor (Variables|Default|GetDoor) false)
  (Audio|PlaySound2D "/Game/Audio/SFX/Elevator/SFX_MISC_Elevator_PowerDown.SFX_MISC_Elevator_PowerDown" 1.0 1.0 0.0 0 0)
  (Class|Shooter|StartNewObjective (Variables|Default|GetShooter) (Utilities|Struct|MakeObjective "Find Engi-26" false "WAYPOINT_Static" 0 0 1e+02 1e+02)))

(fn ConstructionScript)