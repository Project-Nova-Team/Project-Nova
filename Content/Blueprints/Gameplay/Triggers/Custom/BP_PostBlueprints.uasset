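; Custom trigger that cuts the game to black with a sound cue, then loads the NoPower level.
; On activation it casts the activator to BP_Shooter and holds a near-instant camera fade on that player's camera manager.
; It plays a 2D sound and stops the audio components on the Server and RoomTne actors.
; A delay matched to the sound's duration holds the level change until playback ends.
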(event EventTriggerActivated
  (params (Activator :type Pawn%20Object%20Reference))
  (bind _sound (Variables|Default|GetSound))
  (CameraFades|StartCameraFade :self (Variables|/Script/Engine.PlayerController|GetPlayerCameraManager (.AsPlayer%20Controller (Utilities|Casting|CastToPlayerController (Pawn|GetController (.AsBP%20Shooter (Utilities|Casting|CastToBP_Shooter Activator)))))) :ToAlpha 1.0 :Duration 0.01 :bHoldWhenFinished true)
  (Audio|PlaySound2D _sound 1.0 1.0 0.0 0 0)
  (Audio|Components|Audio|Stop (Actor|GetComponentbyClass (Variables|Default|GetServer) "/Script/Engine.AudioComponent"))
  (Audio|Components|Audio|Stop (Actor|GetComponentbyClass (Variables|Default|GetRoomTne) "/Script/Engine.AudioComponent"))
  (Utilities|FlowControl|Delay (Variables|/Script/Engine.SoundBase|GetDuration _sound))
  (Game|OpenLevel(byName) "NoPower"))

(fn ConstructionScript
  (|CallParentFunction))