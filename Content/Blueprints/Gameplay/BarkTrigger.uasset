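; BarkTrigger is a Blueprint that shows and hides an on-screen bark prompt made of prefix, key and suffix text.
; On BeginPlay it adds a BarkPrompt widget to the viewport and binds its handlers to show and hide bark events.
; Showing sets the texts and plays a fade-in.
; Hiding plays a fade-out, whose animation-finished binding collapses the widget.
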(event Custom|SetVisibility
  (Widget|SetVisibility (Variables|Default|GetBarkUI) "Collapsed"))

(event Custom|Hide%20Bark%20UI
  (bind _barkui (Variables|Default|GetBarkUI))
  (UserInterface|Animation|PlayAnimation _barkui (Variables|/Game/Blueprints/UI/BarkPrompt.BarkPrompt_C|GetFadeOut _barkui) 0.0 1 "Forward" 1.0 false))

(event Custom|Show%20Bark%20UI
  (params (PrefixText :type String) (SuffixText :type String) (KeyText :type String))
  (bind _barkui (Variables|Default|GetBarkUI))
  (bind _barkui_2 (Variables|Default|GetBarkUI))
  (Rendering|Components|TextRender|SetText (Variables|/Game/Blueprints/UI/BarkPrompt.BarkPrompt_C|GetPrefixText (Variables|Default|GetBarkUI)) (Utilities|Text|ToText(String) PrefixText))
  (Rendering|Components|TextRender|SetText (Variables|/Game/Blueprints/UI/BarkPrompt.BarkPrompt_C|GetSuffixText (Variables|Default|GetBarkUI)) (Utilities|Text|ToText(String) SuffixText))
  (Rendering|Components|TextRender|SetText (Variables|/Game/Blueprints/UI/BarkPrompt.BarkPrompt_C|GetKeyText _barkui) (Utilities|Text|ToText(String) KeyText))
  (Widget|SetVisibility _barkui "Visible")
  (UserInterface|Animation|PlayAnimation _barkui_2 (Variables|/Game/Blueprints/UI/BarkPrompt.BarkPrompt_C|GetFadeIn _barkui_2) 0.0 1 "Forward" 1.0 false))

(event EventBeginPlay
  (bind _returnvalue (UserInterface|CreateWidget "/Game/Blueprints/UI/BarkPrompt.BarkPrompt_C"))
  (bind _output_get (Variables|Default|SetBarkUI _returnvalue))
  (UserInterface|Viewport|AddtoViewport _output_get 0)
  (EventDispatchers|BindEventtoShowBarkEvent (delegate Custom|Show%20Bark%20UI))
  (EventDispatchers|BindEventtoHideBarkEvent (delegate Custom|Hide%20Bark%20UI))
  (Class|UserWidget|BindtoAnimationFinished (Variables|Default|GetBarkUI) (Variables|/Game/Blueprints/UI/BarkPrompt.BarkPrompt_C|GetFadeOut (Variables|Default|GetBarkUI)) (delegate Custom|SetVisibility)))

(fn ConstructionScript)