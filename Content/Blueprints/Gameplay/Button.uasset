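; Button Blueprint whose mesh glow shows whether it is locked: dark when locked, bright when unlocked.
; The construction script creates a dynamic material instance on the mesh's first material slot.
; BeginPlay applies the initial lock state, and the LockStatusChange event updates the material's Brightness parameter from the status passed in.
; The graph holds no press or interaction logic.
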(event EventBeginPlay
  (if (Variables|Default|GetbIsLocked)
    (Rendering|Material|SetScalarParameterValueonMaterials (Variables|Default|GetButton) "Brightness" 0.0)
    (else
      (Rendering|Material|SetScalarParameterValueonMaterials (Variables|Default|GetButton) "Brightness" 1e+01))))

(event EventLockStatusChange
  (params (LockStatus :type Boolean))
  ;[1 1 1] Set Emissiveness based on lock status
  (if LockStatus
    (Rendering|Material|SetScalarParameterValueonMaterials (Variables|Default|GetButton) "Brightness" 0.0)
    (else
      (Rendering|Material|SetScalarParameterValueonMaterials (Variables|Default|GetButton) "Brightness" 1e+01))))

(fn ConstructionScript
  (bind _returnvalue (Rendering|Material|CreateDynamicMaterialInstance (Variables|Default|GetButton) 0 "/Engine/MapTemplates/Materials/BasicAsset01.BasicAsset01" "None" :!class /Script/Engine.PrimitiveComponent))
  (bind _output_get (Variables|Default|SetDynamicMaterial _returnvalue))
  (Rendering|Material|SetMaterial (Variables|Default|GetButton) 0 _output_get))